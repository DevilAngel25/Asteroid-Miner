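; AsteroidMinerCamera is a player-controlled camera with spring-arm zoom, keyboard movement and mouse rotation.
; Mouse wheel adjusts the boom length within limits, while keyboard axes move the actor along its facing, pinned to world Z zero.
; Holding right mouse opens gates for clamped pitch and free yaw.
; Tick sends position and rotation to DebugHud, then restarts background music on ShipMeshComponent whenever it stops, provided the HUD cast succeeds.
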(event `self.ReceiveTick`
  (params (DeltaSeconds :type "Float (single-precision)"))
  ;[1 1 1] Debug HUD Info
  (set `self.CurrentPosition` (`self.K2_GetActorLocation`))
  (set `self.CurrentRotation` (`self.K2_GetActorRotation`))
  (bind _asdebug_hud (cast `/Game/Blueprints/GameComponents/DebugHud` (`PlayerController.GetHUD` (`GameplayStatics.GetPlayerController` 0))))
  (set `/Game/Blueprints/GameComponents/DebugHud.DisplayVehiclePosition` (`self.CurrentPosition`) _asdebug_hud)
  (set `/Game/Blueprints/GameComponents/DebugHud.DisplayVehicleRotation` (`self.CurrentRotation`) _asdebug_hud)
  ;[1 1 1] Play Background Music
  (bind _returnvalue (`AudioComponent.IsPlaying` (stale _returnvalue_2)))
  (if (not _returnvalue)
    (bind _returnvalue_2 (`GameplayStatics.PlaySoundAttached` "/Game/Audio/BackgroundMusic.BackgroundMusic" (`self.ShipMeshComponent`) "None" (0.0 0.0 0.0) "KeepRelativeOffset" false 1.0 1.0 0.0))))

(event `InputAction|MouseWheelUp`
  ;[1 1 1] Camera Zoom Controls
  (:`Pressed`
    (set `SpringArmComponent.TargetArmLength` (`KismetMathLibrary.FClamp` (- (`SpringArmComponent.TargetArmLength` (`self.CameraBoom`)) (`self.ScrollSensitivity`)) (`self.Min.CameraDistance`) (`self.Max.CameraDistance`)) (`self.CameraBoom`))))

(event `InputAction|MouseWheelDown`
  ;[1 1 1] Camera Zoom Controls
  (:`Pressed`
    (set `SpringArmComponent.TargetArmLength` (`KismetMathLibrary.FClamp` (+ (`SpringArmComponent.TargetArmLength` (`self.CameraBoom`)) (`self.ScrollSensitivity`)) (`self.Min.CameraDistance`) (`self.Max.CameraDistance`)) (`self.CameraBoom`))))

(event `InputAxis|MoveForwardKeyboard`
  (params (AxisValue :type "Float (single-precision)"))
  (bind _returnvalue (`self.GetTransform`))
  ;[1 1 1] Move Camera Forwards and Backwards with Keyboard
  (`self.K2_SetActorTransform` (`KismetMathLibrary.MakeTransform` (`KismetMathLibrary.MakeVector` (.x (+ (`KismetMathLibrary.TransformDirection` _returnvalue (`KismetMathLibrary.MakeVector` (* AxisValue (* (`self.MouseSensitivity`) (`self.MoveSpeed`))))) (.location _returnvalue))) (.y (+ (`KismetMathLibrary.TransformDirection` _returnvalue (`KismetMathLibrary.MakeVector` (* AxisValue (* (`self.MouseSensitivity`) (`self.MoveSpeed`))))) (.location _returnvalue)))) (.rotation _returnvalue) (.scale _returnvalue))))

(event `InputAxis|MoveRightKeyboard`
  (params (AxisValue :type "Float (single-precision)"))
  (bind _returnvalue (`self.GetTransform`))
  ;[1 1 1] Move Camera Left and Right with Keyboard
  (`self.K2_SetActorTransform` (`KismetMathLibrary.MakeTransform` (`KismetMathLibrary.MakeVector` (.x (+ (`KismetMathLibrary.TransformDirection` _returnvalue (`KismetMathLibrary.MakeVector` 0.0 (* AxisValue (* (`self.MouseSensitivity`) (`self.MoveSpeed`))))) (.location _returnvalue))) (.y (+ (`KismetMathLibrary.TransformDirection` _returnvalue (`KismetMathLibrary.MakeVector` 0.0 (* AxisValue (* (`self.MouseSensitivity`) (`self.MoveSpeed`))))) (.location _returnvalue)))) (.rotation _returnvalue) (.scale _returnvalue))))

(event `InputAxisKey|MouseY`
  (params (AxisValue :type "Float (single-precision)"))
  ;[1 1 1] Move Camera in Pitch
  (`/Engine/EditorBlueprintResources/StandardMacros.Gate` true :!label _label
    (:`Exit`
      (`self.SetActorRotation` (`KismetMathLibrary.MakeRot` (`KismetMathLibrary.FClamp` (+ (.pitch (`self.K2_GetActorRotation`)) (* (`self.MouseSensitivity`) AxisValue)) (`self.Min.Pitch`) (`self.Max.Pitch`)) (.yaw (`self.K2_GetActorRotation`)))))))

(event `Key|RightMouseButton`
  ;[1 1 1] Move Camera in Pitch
  (:`Pressed`
    (goto _label :!via `Open`))
  (:`Released`
    (goto _label :!via `Close`)))

(event `InputAxisKey|MouseX`
  (params (AxisValue :type "Float (single-precision)"))
  ;[1 1 1] Move Camera in Yaw
  (`/Engine/EditorBlueprintResources/StandardMacros.Gate` true :!label _label_2
    (:`Exit`
      (`self.SetActorRotation` (`KismetMathLibrary.MakeRot` (.pitch (`self.K2_GetActorRotation`)) (+ (.yaw (`self.K2_GetActorRotation`)) (* (`self.MouseSensitivity`) AxisValue)))))))

(event `Key|RightMouseButton`
  ;[1 1 1] Move Camera in Yaw
  (:`Pressed`
    (goto _label_2 :!via `Open`))
  (:`Released`
    (goto _label_2 :!via `Close`)))

(fn `UserConstructionScript`)