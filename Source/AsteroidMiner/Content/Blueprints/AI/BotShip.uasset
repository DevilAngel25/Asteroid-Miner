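; BotShip is an AI ship actor that reports its state to a debug HUD and is destroyed when it touches the sun.
; Each tick it caches its velocity and pushes that value, along with current and maximum fuel, into the first player controller's DebugHud.
; Overlapping a B_Sun actor destroys the ship; the graphs contain no steering or fuel consumption logic.
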(event `self.ReceiveTick`
  (params (DeltaSeconds :type "Float (single-precision)"))
  ;[1 1 1] Set velocity
  (set `self.CurrentVelocity` (`self.Velocity`))
  ;[1 1 1] Send data to HUD
  (bind _asdebug_hud (cast `/Game/Blueprints/GameComponents/DebugHud` (`PlayerController.GetHUD` (`GameplayStatics.GetPlayerController` 0))))
  (set `/Game/Blueprints/GameComponents/DebugHud.DisplayCurrentFuel` (`self.CurrentFuel`) _asdebug_hud)
  (set `/Game/Blueprints/GameComponents/DebugHud.DisplayVelocityChange` (`self.CurrentVelocity`) _asdebug_hud)
  (set `/Game/Blueprints/GameComponents/DebugHud.MaxFuel` (`self.MaxFuel`) _asdebug_hud)
  (set `/Game/Blueprints/GameComponents/DebugHud.CurrentFuel` (`self.CurrentFuel`) _asdebug_hud))

(event `self.ReceiveActorBeginOverlap`
  (params (OtherActor :type "Actor Object Reference"))
  ;[1 1 1] On collision destroy actor
  (cast `/Game/Blueprints/Objects/B_Sun` OtherActor)
  (`self.K2_DestroyActor`))

(fn `UserConstructionScript`)